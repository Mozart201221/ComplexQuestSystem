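; BP_MasterQuest is the master quest actor of the quest system, tracking a quest's active sub-goals, completed goals and running description.
; Setup functions build current goals from starting indices into QuestInfo, or advance to the index after the highest active one.
; CompleteSubGoal records success, appends description updates and branches into each goal's following sub-goals.
; It also directly updates the quest widget, the journal when this quest is selected there, and sub-goal selection.
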(event EventBeginPlay)

(event Collision|EventActorBeginOverlap
  (params (OtherActor :type Actor%20Object%20Reference)))

(event EventTick
  (params (DeltaSeconds :type Float%20%28single-precision%29)))

(fn ConstructionScript)

(fn -UpdateSubGoals
  (Utilities|Array|Clear (Variables|DoNotTouch!|GetCurrentGoal))
  (for (_ _array_index) (Variables|DoNotTouch!|GetCurrentGoalIndices)
    (Utilities|Array|Add (Variables|DoNotTouch!|GetCurrentGoal) (Utilities|Array|Get(acopy) (Utilities|Struct|BreakS_QuestInfo (Variables|QuestInformation|GetQuestInfo)) _array_index)))
  (return))

(fn -SetupStartingGoals
  (Utilities|Array|Clear (Variables|DoNotTouch!|GetCurrentGoalIndices))
  (Variables|DoNotTouch!|SetCurrentGoalIndices (Variables|QuestInformation|GetStartingSubGoalIndices))
  (CallFunction|-UpdateSubGoals)
  (Variables|DoNotTouch!|SetCurrentDescription (.Description (Utilities|Struct|BreakS_QuestInfo (Variables|QuestInformation|GetQuestInfo))))
  (return))

(fn -GotoNextSubGoals
  (bind _currentgoalindices (Variables|DoNotTouch!|GetCurrentGoalIndices))
  (bind _currentgoalindices_2 (Variables|DoNotTouch!|GetCurrentGoalIndices))
  (bind _maxvalue (Math|Integer|MaxOfIntArray _currentgoalindices))
  (bind _returnvalue (+ _maxvalue 1))
  (if (<= _returnvalue (Utilities|Array|Length (.SubGoals (Utilities|Struct|BreakS_QuestInfo (Variables|QuestInformation|GetQuestInfo)))))
    (LocalVariables|SetL_NextIndex _returnvalue)
    (Utilities|Array|Clear _currentgoalindices_2)
    (Utilities|Array|Add _currentgoalindices_2 (LocalVariables|GetL_NextIndex))
    (CallFunction|-UpdateSubGoals)
    (return true)
    (else
      (return false))))

(fn -CompleteSubGoal
  (params (SubGoalIndex :type Integer))
  (bind _questwidget (Variables|DoNotTouch!|GetQuestWidget))
  (bind _questwidget_2 (Variables|DoNotTouch!|GetQuestWidget))
  (bind _questwidget_3 (Variables|DoNotTouch!|GetQuestWidget))
  (bind _currentgoalindices (Variables|DoNotTouch!|GetCurrentGoalIndices))
  (bind _subgoalwidget (Variables|/Game/QuestSystem/Widgets/W_QuestWidget.W_QuestWidget_C|GetSubGoalWidget _questwidget))
  (LocalVariables|SetLocalGoalIndex SubGoalIndex)
  (if (Utilities|Array|ContainsItem (Variables|DoNotTouch!|GetCurrentGoalIndices) (LocalVariables|GetLocalGoalIndex))
    (bind _output_get (LocalVariables|SetLocalCompletedGoal (Utilities|Array|Get(acopy) (Utilities|Struct|BreakS_QuestInfo (Variables|QuestInformation|GetQuestInfo)) (LocalVariables|GetLocalGoalIndex))))
    (Utilities|Array|Add (Variables|DoNotTouch!|GetCompletedSubGoals) (Utilities|Struct|MakeS_CompletedGoal (LocalVariables|GetLocalGoalIndex) _output_get true))
    (if (.UpdateQuestDescription? (Utilities|Struct|BreakS_GoalInfo (LocalVariables|GetLocalCompletedGoal)))
      (Variables|DoNotTouch!|SetCurrentDescription (Utilities|Text|FormatText "{Current}{Next}" (Variables|DoNotTouch!|GetCurrentDescription) (.UpdateDescription (Utilities|Struct|BreakS_GoalInfo (LocalVariables|GetLocalCompletedGoal)))))
      (if (CallFunction|-SelectedinJournal?)
        (Default|-UpdateDescription (Variables|/Game/QuestSystem/Widgets/-W_MainWidget.-W_MainWidget_C|GetW_QuestJournal (Variables|/Game/QuestSystem/Blueprints/Actors/BP_QuestManager.BP_QuestManager_C|GetMainWidget (Variables|DoNotTouch!|GetQuestManager))))))
    (Utilities|Array|RemoveItem (Variables|DoNotTouch!|GetCurrentGoal) (LocalVariables|GetLocalCompletedGoal))
    (LocalVariables|SetlocalWidgetIndex (Utilities|Array|FindItem _currentgoalindices (LocalVariables|GetLocalGoalIndex)))
    (Utilities|Array|RemoveItem _currentgoalindices (LocalVariables|GetLocalGoalIndex))
    (Widget|RemovefromParent (Utilities|Array|Get(acopy) _subgoalwidget (LocalVariables|GetLocalGoalIndex)))
    (Utilities|Array|RemoveIndex _subgoalwidget (LocalVariables|GetlocalWidgetIndex))
    (for _array_element (Utilities|Struct|BreakS_GoalInfo (LocalVariables|GetLocalCompletedGoal))
      (Utilities|Array|Add (Variables|DoNotTouch!|GetCurrentGoalIndices) _array_element)
      (Utilities|Array|Add (Variables|DoNotTouch!|GetCurrentGoal) (Utilities|Array|Get(acopy) (.SubGoals (Utilities|Struct|BreakS_QuestInfo (Variables|QuestInformation|GetQuestInfo))) _array_element))
      (bind _returnvalue (UserInterface|CreateWidget "/Game/QuestSystem/Widgets/W_SubGoalWidget.W_SubGoalWidget_C" 0 (Utilities|Array|Get(acopy) (.SubGoals (Utilities|Struct|BreakS_QuestInfo (Variables|QuestInformation|GetQuestInfo))) _array_element) self (Variables|DoNotTouch!|GetQuestWidget)))
      (Utilities|Array|Add (Variables|/Game/QuestSystem/Widgets/W_QuestWidget.W_QuestWidget_C|GetSubGoalWidget _questwidget_2) _returnvalue)
      (Widget|Panel|AddChild (Variables|/Game/QuestSystem/Widgets/W_QuestWidget.W_QuestWidget_C|GetSubGoalBox _questwidget_2) _returnvalue))
    (if (CallFunction|-SelectedinJournal?)
      (Default|-GenerateSubGoals (Variables|/Game/QuestSystem/Widgets/-W_MainWidget.-W_MainWidget_C|GetW_QuestJournal (Variables|/Game/QuestSystem/Blueprints/Actors/BP_QuestManager.BP_QuestManager_C|GetMainWidget (Variables|DoNotTouch!|GetQuestManager)))))
    (if (and (== (LocalVariables|GetLocalGoalIndex) (Variables|DoNotTouch!|GetSelectedSubGoalIndex)) (== (Variables|/Game/QuestSystem/Blueprints/Actors/BP_QuestManager.BP_QuestManager_C|GetCurrentQuest (Variables|DoNotTouch!|GetQuestManager)) self))
      (Default|-SelectSubGoal _questwidget_3 (Utilities|Array|Get(acopy) (Variables|/Game/QuestSystem/Widgets/W_QuestWidget.W_QuestWidget_C|GetSubGoalWidget _questwidget_3)))
      (return true)
      (else
        (return true)))
    (else
      (return false))))

(fn -SelectedinJournal?
  (bind _questmanager (Variables|DoNotTouch!|GetQuestManager))
  (bind _mainwidget (Variables|/Game/QuestSystem/Blueprints/Actors/BP_QuestManager.BP_QuestManager_C|GetMainWidget _questmanager))
  (bind _w_questjournal (Variables|/Game/QuestSystem/Widgets/-W_MainWidget.-W_MainWidget_C|GetW_QuestJournal _mainwidget))
  (bind _selectedquest (Variables|/Game/QuestSystem/Widgets/W_QuestJournal.W_QuestJournal_C|GetSelectedQuest _w_questjournal))
  (return (and (Utilities|IsValid _selectedquest) (== _selectedquest self))))