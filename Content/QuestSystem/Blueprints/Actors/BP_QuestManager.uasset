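; BP_QuestManager is the quest system's central actor, spawning unique quest actors and linking them to the HUD list and journal.
; NPC talk, object found and enemy kill events match each active quest's current goals to complete subgoals or advance hunt counts.
; Switching subgoals respawns a goal actor at any set location.
; Player movement updates its 2D distance and minimap arrow, using paired DoOnce gates to toggle arrow visibility at a threshold.
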(event Custom|OnSwitchSubQuest
  (bind _currentquest (Variables|Default|GetCurrentQuest))
  (bind _mainwidget (Variables|Default|GetMainWidget))
  (Utilities|IsValid (Variables|Default|GetCurrentGoalActor)
    (:Is%20Valid
      (Actor|DestroyActor (Variables|Default|GetCurrentGoalActor)))
    (:Is%20Not%20Valid
      _))
  (bind _output_get (Variables|Default|SetCurrentSubGoal (Utilities|Array|Get(acopy) (Utilities|Struct|BreakS_QuestInfo (Variables|/Game/QuestSystem/Blueprints/Actors/QuestActors/BP_MasterQuest.BP_MasterQuest_C|GetQuestInfo _currentquest)) (Variables|/Game/QuestSystem/Blueprints/Actors/QuestActors/BP_MasterQuest.BP_MasterQuest_C|GetSelectedSubGoalIndex _currentquest))))
  (if (.HasLocation? (Utilities|Struct|BreakS_GoalLocation (.GoalLocation (Utilities|Struct|BreakS_GoalInfo _output_get))))
    (bind _returnvalue (Game|SpawnActorfromClass "/Game/QuestSystem/Blueprints/Actors/BP_GoalActor.BP_GoalActor_C" (Math|Transform|MakeTransform (.Location (Utilities|Struct|BreakS_GoalLocation (.GoalLocation (Utilities|Struct|BreakS_GoalInfo _output_get)))) "0, 0, 0" "1,1,1") "AlwaysSpawn" 0 (.UseRadius? (Utilities|Struct|BreakS_GoalInfo _output_get)) (.Radius (Utilities|Struct|BreakS_GoalInfo _output_get)) (.CircleColor (Utilities|Struct|BreakS_GoalInfo _output_get)) 0))
    (Variables|Default|SetCurrentGoalActor _returnvalue)
    (bind _output_get_2 (Variables|Default|SetCurrentDistance (CallFunction|-DistancetoGoal)))
    (Rendering|Components|TextRender|SetText (Variables|/Game/QuestSystem/Widgets/-W_MainWidget.-W_MainWidget_C|GetDistanceText (Variables|Default|GetMainWidget)) (Utilities|Text|ToText(Integer) _output_get_2 false false))
    (CallFunction|-UpdateDirectionArrow)
    (Widget|SetVisibility (Variables|/Game/QuestSystem/Widgets/-W_MainWidget.-W_MainWidget_C|GetDistanceBorder _mainwidget) "HitTestInvisible")
    (Widget|SetVisibility (Variables|/Game/QuestSystem/Widgets/W_MiniMap.W_MiniMap_C|GetDirectionArrow (Variables|/Game/QuestSystem/Widgets/-W_MainWidget.-W_MainWidget_C|GetW_MiniMap _mainwidget)) (select (> (Variables|Default|GetCurrentDistance) (Variables|Default|GetShowDirectionArrowAmount)) "HitTestInvisible" "Hidden"))
    (else
      (Variables|Default|SetCurrentGoalActor 0)
      (Widget|SetVisibility (Variables|/Game/QuestSystem/Widgets/-W_MainWidget.-W_MainWidget_C|GetDistanceBorder (Variables|Default|GetMainWidget)) "Hidden"))))

(event Custom|OnPlayerMove
  (Utilities|IsValid (Variables|Default|GetCurrentGoalActor)
    (:Is%20Valid
      (bind _output_get (Variables|Default|SetCurrentDistance (CallFunction|-DistancetoGoal)))
      (Rendering|Components|TextRender|SetText (Variables|/Game/QuestSystem/Widgets/-W_MainWidget.-W_MainWidget_C|GetDistanceText (Variables|Default|GetMainWidget)) (Utilities|Text|ToText(Integer) _output_get false false))
      (Math|Integer|CompareInt (Variables|Default|GetCurrentDistance) (Variables|Default|GetShowDirectionArrowAmount)
        (:>
          _)
        (:==
          _)
        (:<
          (Utilities|FlowControl|DoOnce false :!label _label
            (:Completed
              (Widget|SetVisibility (Variables|/Game/QuestSystem/Widgets/W_MiniMap.W_MiniMap_C|GetDirectionArrow (Variables|/Game/QuestSystem/Widgets/-W_MainWidget.-W_MainWidget_C|GetW_MiniMap (Variables|Default|GetMainWidget))) "Hidden")
              (goto _label_2 Reset)))))
      (CallFunction|-UpdateDirectionArrow)
      (Utilities|FlowControl|DoOnce false :!label _label_2
        (:Completed
          (Widget|SetVisibility (Variables|/Game/QuestSystem/Widgets/W_MiniMap.W_MiniMap_C|GetDirectionArrow (Variables|/Game/QuestSystem/Widgets/-W_MainWidget.-W_MainWidget_C|GetW_MiniMap (Variables|Default|GetMainWidget))) "HitTestInvisible")
          (goto _label Reset))))))

(event Custom|OnEnemyKilled
  (params (Class :type Master%20Enemy%20Class%20Reference))
  (Variables|Default|SetKilledEnemy Class)
  ;[1 1 1] На EventBeginPlay добавить инициализацию переменных FindCurrentQuestActor и FindCurrentGoalIndex с ForEachLoop
  (for _array_element (Variables|Default|GetCurrentQuestActors)
    (bind _output_get (Variables|Default|SetFindCurrentQuestActor _array_element))
    (for (_array_element_2 _array_index) (Variables|/Game/QuestSystem/Blueprints/Actors/QuestActors/BP_MasterQuest.BP_MasterQuest_C|GetCurrentGoal _output_get)
      (Variables|Default|SetFindCurrentGoalIndex _array_index)
      (if (and (Utilities|Enum|Equal(Enum) (.Type (Utilities|Struct|BreakS_GoalInfo _array_element_2)) "NewEnumerator1") (== (.GoalClass (Utilities|Struct|BreakS_GoalInfo _array_element_2)) (Variables|Default|GetKilledEnemy)))
        (if (>= (+ (Utilities|Array|Get(acopy) (Variables|/Game/QuestSystem/Blueprints/Actors/QuestActors/BP_MasterQuest.BP_MasterQuest_C|GetCurrentHuntedAmounts (Variables|Default|GetFindCurrentQuestActor)) (Variables|Default|GetFindCurrentGoalIndex)) 1) (.AmountToHunt (Utilities|Struct|BreakS_GoalInfo _array_element_2)))
          (Default|-CompleteSubGoal (Variables|Default|GetFindCurrentQuestActor) (Utilities|Array|Get(acopy) (Variables|/Game/QuestSystem/Blueprints/Actors/QuestActors/BP_MasterQuest.BP_MasterQuest_C|GetCurrentGoalIndices (Variables|Default|GetFindCurrentQuestActor)) (Variables|Default|GetFindCurrentGoalIndex)))
          (else
            (Utilities|Array|SetArrayElem (Variables|/Game/QuestSystem/Blueprints/Actors/QuestActors/BP_MasterQuest.BP_MasterQuest_C|GetCurrentHuntedAmounts (Variables|Default|GetFindCurrentQuestActor)) (Variables|Default|GetFindCurrentGoalIndex) (+ (Utilities|Array|Get(acopy) (Variables|/Game/QuestSystem/Blueprints/Actors/QuestActors/BP_MasterQuest.BP_MasterQuest_C|GetCurrentHuntedAmounts (Variables|Default|GetFindCurrentQuestActor)) (Variables|Default|GetFindCurrentGoalIndex)) 1))
            (Default|-Update (Utilities|Array|Get(acopy) (Variables|/Game/QuestSystem/Widgets/W_QuestWidget.W_QuestWidget_C|GetSubGoalWidget (Variables|/Game/QuestSystem/Blueprints/Actors/QuestActors/BP_MasterQuest.BP_MasterQuest_C|GetQuestWidget (Variables|Default|GetFindCurrentQuestActor))) (Variables|Default|GetFindCurrentGoalIndex)))
            (if (Default|-SelectedinJournal? (Variables|Default|GetFindCurrentQuestActor))
              (Default|-GenerateSubGoals (Variables|/Game/QuestSystem/Widgets/-W_MainWidget.-W_MainWidget_C|GetW_QuestJournal (Variables|Default|GetMainWidget))))))))))

(event Custom|OnObjectFound
  (params (FoundObject :type Master%20Object%20Class%20Reference))
  (Variables|Default|SetFoundObject FoundObject)
  ;[1 1 1] На EventBeginPlay добавить инициализацию переменных FindCurrentQuestActor и FindCurrentGoalIndex с ForEachLoop
  (for _array_element (Variables|Default|GetCurrentQuestActors)
    (for (_array_element_2 _array_index) (Variables|/Game/QuestSystem/Blueprints/Actors/QuestActors/BP_MasterQuest.BP_MasterQuest_C|GetCurrentGoal _array_element)
      (if (and (Utilities|Enum|Equal(Enum) (.Type (Utilities|Struct|BreakS_GoalInfo _array_element_2)) "NewEnumerator2") (== (.GoalClass (Utilities|Struct|BreakS_GoalInfo _array_element_2)) (Variables|Default|GetFoundObject)))
        (Default|-CompleteSubGoal _array_element (Utilities|Array|Get(acopy) (Variables|/Game/QuestSystem/Blueprints/Actors/QuestActors/BP_MasterQuest.BP_MasterQuest_C|GetCurrentGoalIndices _array_element) _array_index))))))

(event Custom|OnTalkToNPC
  (params (NPCClass :type Master%20NPC%20Class%20Reference) (NPCID :type Integer))
  (for _array_element (Variables|Default|GetCurrentQuestActors)
    (for (_array_element_2 _array_index) (Variables|/Game/QuestSystem/Blueprints/Actors/QuestActors/BP_MasterQuest.BP_MasterQuest_C|GetCurrentGoal _array_element)
      (if (Math|Boolean|ANDBoolean (Utilities|Enum|Equal(Enum) (.Type (Utilities|Struct|BreakS_GoalInfo _array_element_2)) "NewEnumerator3") (== (.GoalClass (Utilities|Struct|BreakS_GoalInfo _array_element_2)) NPCClass) (== (.GoalID (Utilities|Struct|BreakS_GoalInfo _array_element_2)) NPCID))
        (Default|-CompleteSubGoal _array_element (Utilities|Array|Get(acopy) (Variables|/Game/QuestSystem/Blueprints/Actors/QuestActors/BP_MasterQuest.BP_MasterQuest_C|GetCurrentGoalIndices _array_element) _array_index))))))

(event EventBeginPlay
  ;[1 1 1] На EventBeginPlay добавить инициализацию переменных FindCurrentQuestActor и FindCurrentGoalIndex с ForEachLoop
)

(fn ConstructionScript)

(fn -SelectNewQuest
  (params (Quest :type BP%20Master%20Quest%20Object%20Reference) (SubGoal :type W%20Sub%20Goal%20Widget%20Object%20Reference))
  (Utilities|IsValid (Variables|Default|GetCurrentQuest)
    (:Is%20Valid
      (Widget|SetIsEnabled (Variables|/Game/QuestSystem/Widgets/W_QuestWidget.W_QuestWidget_C|GetQuestName (Variables|/Game/QuestSystem/Blueprints/Actors/QuestActors/BP_MasterQuest.BP_MasterQuest_C|GetQuestWidget (Variables|Default|GetCurrentQuest))) false)
      (Default|-SelectSubGoal (Variables|/Game/QuestSystem/Blueprints/Actors/QuestActors/BP_MasterQuest.BP_MasterQuest_C|GetQuestWidget (Variables|Default|GetCurrentQuest))))
    (:Is%20Not%20Valid
      _))
  (bind _output_get (Variables|Default|SetCurrentQuest Quest))
  (Default|-SelectSubGoal (Variables|/Game/QuestSystem/Blueprints/Actors/QuestActors/BP_MasterQuest.BP_MasterQuest_C|GetQuestWidget _output_get) SubGoal)
  (return))

(fn -AddNewQuest
  (params (QuestClass :type BP%20Master%20Quest%20Class%20Reference) (DirectlyStart? :type Boolean))
  (bind _mainwidget (Variables|Default|GetMainWidget))
  (LocalVariables|SetL_QuestClass QuestClass)
  (LocalVariables|SetL_DirectlyStart DirectlyStart?)
  (if (and (Utilities|IsValidClass QuestClass) (not (Utilities|Array|ContainsItem (Variables|Default|GetAllQuestClasses) QuestClass)))
    (Utilities|Array|Add (Variables|Default|GetAllQuestClasses) (LocalVariables|GetL_QuestClass))
    (bind _returnvalue (Game|SpawnActorfromClass (LocalVariables|GetL_QuestClass) (Math|Transform|MakeTransform "0, 0, 0" "0, 0, 0" "1,1,1") "AlwaysSpawn" 0 self 0))
    (bind _output_get (LocalVariables|SetL_QuestActor _returnvalue))
    (Utilities|Array|Add (Variables|Default|GetCurrentQuestActors) _output_get)
    (bind _widget (Default|-AddQuesttoList (Variables|Default|GetMainWidget) (LocalVariables|GetL_QuestActor)))
    (bind _output_get_2 (Variables|/Game/QuestSystem/Blueprints/Actors/QuestActors/BP_MasterQuest.BP_MasterQuest_C|SetQuestWidget (LocalVariables|GetL_QuestActor) _widget))
    (Default|-SetupStartingGoals (LocalVariables|GetL_QuestActor))
    (Default|-UpdateQuest _output_get_2)
    (Default|-AddEntry (Variables|/Game/QuestSystem/Widgets/-W_MainWidget.-W_MainWidget_C|GetW_QuestJournal (Variables|Default|GetMainWidget)) (LocalVariables|GetL_QuestActor))
    (if (or (LocalVariables|GetL_DirectlyStart) (<= (Utilities|Array|Length (Variables|Default|GetCurrentQuestActors)) 1))
      (CallFunction|-SelectNewQuest (LocalVariables|GetL_QuestActor) (Utilities|Array|Get(acopy) (Variables|/Game/QuestSystem/Widgets/W_QuestWidget.W_QuestWidget_C|GetSubGoalWidget (Variables|/Game/QuestSystem/Blueprints/Actors/QuestActors/BP_MasterQuest.BP_MasterQuest_C|GetQuestWidget (LocalVariables|GetL_QuestActor))))))
    (if (Variables|/Game/QuestSystem/Widgets/-W_MainWidget.-W_MainWidget_C|GetSlideOut? (Variables|Default|GetMainWidget))
      (UserInterface|Animation|PlayAnimation _mainwidget (Variables|/Game/QuestSystem/Widgets/-W_MainWidget.-W_MainWidget_C|GetSlideOut _mainwidget) 0.0 1 "Reverse" 1.0 false)
      (Variables|/Game/QuestSystem/Widgets/-W_MainWidget.-W_MainWidget_C|SetSlideOut? _mainwidget false)
      (return true)
      (else
        (return true)))
    (else
      (return false))))

(fn -DistancetoGoal
  (bind _thirdpersonchar (Variables|Default|GetThirdPersonChar))
  (bind _currentgoalactor (Variables|Default|GetCurrentGoalActor))
  (bind _returnvalue (Transformation|GetActorLocation _thirdpersonchar))
  (bind _returnvalue_2 (Transformation|GetActorLocation _currentgoalactor))
  (return (Math|Float|Round (/ (Math|Vector|VectorLength (- (Math|Vector|MakeVector (.x _returnvalue) (.y _returnvalue) 0.0) (Math|Vector|MakeVector (.x _returnvalue_2) (.y _returnvalue_2) 0.0))) 1e+02))))

(fn -UpdateDirectionArrow
  (Class|Widget|SetRenderTransformAngle (Variables|/Game/QuestSystem/Widgets/W_MiniMap.W_MiniMap_C|GetDirectionArrow (Variables|/Game/QuestSystem/Widgets/-W_MainWidget.-W_MainWidget_C|GetW_MiniMap (Variables|Default|GetMainWidget))) (.Yaw (Math|Rotator|BreakRotator (Math|Rotator|FindLookatRotation (Transformation|GetActorLocation (Variables|Default|GetThirdPersonChar)) (Transformation|GetActorLocation (Variables|Default|GetCurrentGoalActor))))))
  (return))

(fn -HasCurrentQuest?
  (params (QuestClass :type BP%20Master%20Quest%20Class%20Reference))
  (bind _array_element (Utilities|Array|ForEachLoopwithBreak (Variables|Default|GetCurrentQuestActors) :!label _label)
    (:LoopBody
      (if (== (Utilities|GetClass _array_element) QuestClass)
        (LocalVariables|SetL_FoundQuest _array_element)
        (goto _label Break)))
    (:Completed
      (Utilities|IsValid (LocalVariables|GetL_FoundQuest)
        (:Is%20Valid
          (return true (LocalVariables|GetL_FoundQuest)))
        (:Is%20Not%20Valid
          (return false 0))))))