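; NPC Blueprint for a quest giver that offers its quest only when the player's prestige in a given region meets a required threshold.
; It checks prestige on quest load and on prestige gain, showing a question mark while the quest is available.
; Interacting adds and starts the quest, hides the marker and switches to a post-quest message; otherwise the parent interaction runs.
; On load, a quest already in the manager marks it as given.
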(event EventBeginPlay
  (|CallParentFunction) ; This node is disabled and will not be called.\nDrag off pins to build functionality.
)

(event EventOnPlayerGainPrestige
  (params (Player :type Third%20Person%20Character%20Object%20Reference))
  (bind _requiredprestige (Variables|Default|GetRequiredPrestige))
  (bind (_region _prestige) (Utilities|Struct|BreakS_RegionPrestige _requiredprestige))
  (if (Math|Boolean|ANDBoolean (>= (Default|-GetPrestigebyRegion Player _region) _prestige) (not (Variables|Default|GetCanGiveQuest?)) (not (Variables|Default|GetHasGivenQuest?)))
    (Variables|Default|SetCanGiveQuest? true)
    (Rendering|SetVisibility (Variables|Default|GetQuestionMark) true false)))

(event EventOnQuestLoaded
  (params (Manager :type BP%20Quest%20Manager%20Object%20Reference))
  (bind _requiredprestige (Variables|Default|GetRequiredPrestige))
  (bind (_region _prestige) (Utilities|Struct|BreakS_RegionPrestige _requiredprestige))
  (if (>= (Default|-GetPrestigebyRegion (Variables|/Game/QuestSystem/Blueprints/Actors/BP_QuestManager.BP_QuestManager_C|GetThirdPersonChar Manager) _region) _prestige)
    (Variables|Default|SetCanGiveQuest? true)
    (if (Utilities|Array|ContainsItem (Variables|/Game/QuestSystem/Blueprints/Actors/BP_QuestManager.BP_QuestManager_C|GetAllQuestClasses Manager) (Variables|Default|GetQuestToGive))
      (Variables|Default|SetHasGivenQuest? true)
      (Variables|Default|SetDefaultMessage (Variables|Default|GetMsgAfterQuestGiven))
      (else
        (Rendering|SetVisibility (Variables|Default|GetQuestionMark) true false)))))

(event EventOnInteractwith
  (params (Character :type Third%20Person%20Character%20Object%20Reference))
  (if (and (Variables|Default|GetCanGiveQuest?) (not (Variables|Default|GetHasGivenQuest?)))
    (Default|-AddNewQuest (Variables|/Game/QuestSystem/Blueprints/Characters/ThirdPersonCharacter.ThirdPersonCharacter_C|GetQuestManagerRef Character) (Variables|Default|GetQuestToGive) true)
    (Variables|Default|SetHasGivenQuest? true)
    (Variables|Default|SetDefaultMessage (Variables|Default|GetMsgAfterQuestGiven))
    (Rendering|SetVisibility (Variables|Default|GetQuestionMark) false false)
    (else
      (|CallParentFunction Character))))

(fn ConstructionScript
  (|CallParentFunction))